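; Castle guard enemy Blueprint for a side-scroller, handling both player character classes.
; HitBox overlaps knock players sideways and damage them unless they hold a pickup, while falling BoxJump overlaps bounce them and reduce guard health, updating its bar.
; At low health, Tick counts the kill once in achievements, stats and GameInstance, then sets pawn collision to overlap without destroying the actor.
; Later BoxJump overlaps add achievement and stat progress again.
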(event OnComponentBeginOverlap(BoxJump)
  (params (OverlappedComponent :type Primitive%20Component%20Object%20Reference) (OtherActor :type Actor%20Object%20Reference) (OtherComp :type Primitive%20Component%20Object%20Reference) (OtherBodyIndex :type Integer) (bFromSweep :type Boolean) (SweepResult :type Hit%20Result%20Structure%20%28by%20ref%29))
  (bind _hurtsound (Variables|Default|GetHurtSound))
  (bind _asside_scroller_character (Utilities|Casting|CastToSideScrollerCharacter OtherActor)
    (:then
      (if (> (Variables|Default|GetHealth) 0.2)
        (if (AI|Components|NavMovement|IsFalling (Variables|/Script/Engine.Character|GetCharacterMovement _asside_scroller_character))
          (if (>= (.y (Transformation|GetWorldLocation (Variables|/Script/Engine.Character|GetCapsuleComponent _asside_scroller_character))) (.y (Transformation|GetWorldLocation (Variables|Collision|GetCapsuleComponent))))
            (Variables|Default|SetPush "0,1100.000000, 0")
            (else
              (Variables|Default|SetPush "0,-1100.000000, 0")))
          (Variables|/Script/Engine.MovementComponent|SetVelocity (Variables|/Script/Engine.Character|GetCharacterMovement _asside_scroller_character) (Variables|Default|GetPush))
          (Variables|Default|SetHealth (- (Variables|Default|GetHealth) 0.2) :!label _label)
          (bind _asenemy_health_bar (Utilities|Casting|CastToEnemyHealthBar (UserInterface|GetUserWidgetObject (Variables|Default|GetHealthBar))))
          (Progress|SetPercent (Variables|/Game/GameUI/EnemyHealthBar.EnemyHealthBar_C|GetBar _asenemy_health_bar) (Variables|Default|GetHealth))
          (Utilities|IsValid _hurtsound
            (:Is%20Valid
              (Audio|Components|Audio|Play _hurtsound 0.0))))
        (else
          (Class|AchievementSubSystem|AddAchievementProgress (Subsystems|GetAchievementSubSystem) "Enemies" 1.0)
          (CallFunction|AddActivePlayerStats 0.0 1))))
    (:CastFailed
      (bind _asside_scroller_character_2 (Utilities|Casting|CastToSideScrollerCharacter_2 OtherActor))
      (if (> (Variables|Default|GetHealth) 0.2)
        (if (AI|Components|NavMovement|IsFalling (Variables|/Script/Engine.Character|GetCharacterMovement _asside_scroller_character_2))
          (if (>= (.y (Transformation|GetWorldLocation (Variables|/Script/Engine.Character|GetCapsuleComponent _asside_scroller_character_2))) (.y (Transformation|GetWorldLocation (Variables|Collision|GetCapsuleComponent))))
            (Variables|Default|SetPush "0,1100.000000, 0")
            (else
              (Variables|Default|SetPush "0,-1100.000000, 0")))
          (Variables|/Script/Engine.MovementComponent|SetVelocity (Variables|/Script/Engine.Character|GetCharacterMovement _asside_scroller_character_2) (Variables|Default|GetPush))
          (goto _label))
        (else
          (Class|AchievementSubSystem|AddAchievementProgress (Subsystems|GetAchievementSubSystem) "Enemies" 1.0)
          (CallFunction|AddActivePlayerStats 0.0 1))))))

(event OnComponentBeginOverlap(HitBox)
  (params (OverlappedComponent :type Primitive%20Component%20Object%20Reference) (OtherActor :type Actor%20Object%20Reference) (OtherComp :type Primitive%20Component%20Object%20Reference) (OtherBodyIndex :type Integer) (bFromSweep :type Boolean) (SweepResult :type Hit%20Result%20Structure%20%28by%20ref%29))
  (if (> (Variables|Default|GetHealth) 0.2)
    (bind _asside_scroller_character (Utilities|Casting|CastToSideScrollerCharacter OtherActor)
      (:then
        (if (>= (.y (Transformation|GetWorldLocation (Variables|/Script/Engine.Character|GetCapsuleComponent _asside_scroller_character))) (.y (Transformation|GetWorldLocation (Variables|Collision|GetCapsuleComponent))))
          (Variables|Default|SetPush "0,3000.000000, 0")
          (else
            (Variables|Default|SetPush "0,-3000.000000, 0")))
        (Variables|/Script/Engine.MovementComponent|SetVelocity (Variables|/Script/Engine.Character|GetCharacterMovement _asside_scroller_character) (Variables|Default|GetPush))
        (if (> (Variables|/Game/SideScrollerCPP/Blueprints/SideScrollerCharacter.SideScrollerCharacter_C|GetHealth _asside_scroller_character) 0.0)
          (if (not (Variables|/Game/SideScrollerCPP/Blueprints/SideScrollerCharacter.SideScrollerCharacter_C|GethasPickUp _asside_scroller_character))
            (Variables|/Game/SideScrollerCPP/Blueprints/SideScrollerCharacter.SideScrollerCharacter_C|SetHealth _asside_scroller_character (- (Variables|/Game/SideScrollerCPP/Blueprints/SideScrollerCharacter.SideScrollerCharacter_C|GetHealth _asside_scroller_character) 1e+01)))))
      (:CastFailed
        (bind _asside_scroller_character_2 (Utilities|Casting|CastToSideScrollerCharacter_2 OtherActor))
        (if (>= (.y (Transformation|GetWorldLocation (Variables|/Script/Engine.Character|GetCapsuleComponent _asside_scroller_character_2))) (.y (Transformation|GetWorldLocation (Variables|Collision|GetCapsuleComponent))))
          (Variables|Default|SetPush "0,3000.000000, 0")
          (else
            (Variables|Default|SetPush "0,-3000.000000, 0")))
        (Variables|/Script/Engine.MovementComponent|SetVelocity (Variables|/Script/Engine.Character|GetCharacterMovement _asside_scroller_character_2) (Variables|Default|GetPush))
        (if (> (Variables|/Game/SideScrollerCPP/Blueprints/SideScrollerCharacter_2.SideScrollerCharacter_2_C|GetHealth _asside_scroller_character_2) 0.0)
          (if (not (Variables|/Game/SideScrollerCPP/Blueprints/SideScrollerCharacter_2.SideScrollerCharacter_2_C|GethasPickUp _asside_scroller_character_2))
            (Variables|/Game/SideScrollerCPP/Blueprints/SideScrollerCharacter_2.SideScrollerCharacter_2_C|SetHealth _asside_scroller_character_2 (- (Variables|/Game/SideScrollerCPP/Blueprints/SideScrollerCharacter_2.SideScrollerCharacter_2_C|GetHealth _asside_scroller_character_2) 1e+01))))))))

(event EventOnJumped)

(event EventTick
  (params (DeltaSeconds :type Float%20%28single-precision%29))
  (if (not (> (Variables|Default|GetHealth) 0.2))
    (if (not (Variables|Default|GetAlreadyCheacked))
      (Variables|Default|SetAlreadyCheacked true)
      (Class|AchievementSubSystem|AddAchievementProgress (Subsystems|GetAchievementSubSystem) "Enemies" 1.0)
      (CallFunction|AddActivePlayerStats 0.0 1)
      (bind _asgame_instance_bp (Utilities|Casting|CastToGameInstanceBP (Game|GetGameInstance)))
      (bind _output_get (Variables|/Game/SideScrollerCPP/Blueprints/GameInstanceBP.GameInstanceBP_C|SetEnemies _asgame_instance_bp (+ (Variables|/Game/SideScrollerCPP/Blueprints/GameInstanceBP.GameInstanceBP_C|GetEnemies _asgame_instance_bp) 1)))
      (Development|PrintString (Utilities|String|ToString(Integer) _output_get))
      (Collision|SetCollisionResponsetoChannel (Variables|Collision|GetCapsuleComponent) "ECC_Pawn" "ECR_Overlap"))))

(fn ConstructionScript)

(fn Flicker)