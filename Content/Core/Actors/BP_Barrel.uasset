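; Barrel hazard for the side-scroller that hurts player characters and can optionally spin or show spikes.
; Box overlap subtracts health from either character class and plays a damage sound created at BeginPlay, regardless of spike visibility.
; The first capsule hit by SideScrollerCharacter adds "Barrel" achievement progress; the SideScrollerCharacter_2 path is unwired.
; Construction script sets spike visibility, and Tick applies a frame-rate-dependent rotation when CanRotate is set.
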(event OnComponentBeginOverlap(Box)
  (params (OverlappedComponent :type Primitive%20Component%20Object%20Reference) (OtherActor :type Actor%20Object%20Reference) (OtherComp :type Primitive%20Component%20Object%20Reference) (OtherBodyIndex :type Integer) (bFromSweep :type Boolean) (SweepResult :type Hit%20Result%20Structure%20%28by%20ref%29))
  (bind _s_ound (Variables|Default|GetS%20OUND))
  (bind _s_ound_2 (Variables|Default|GetS%20OUND))
  (bind _asside_scroller_character (Utilities|Casting|CastToSideScrollerCharacter OtherActor)
    (:then
      (Variables|/Game/SideScrollerCPP/Blueprints/SideScrollerCharacter.SideScrollerCharacter_C|SetHealth _asside_scroller_character (- (Variables|/Game/SideScrollerCPP/Blueprints/SideScrollerCharacter.SideScrollerCharacter_C|GetHealth _asside_scroller_character) 1e+01))
      (Development|PrintString "Hello")
      (Utilities|IsValid _s_ound
        (:Is%20Valid
          (Audio|Components|Audio|Play _s_ound 0.0))))
    (:CastFailed
      (bind _asside_scroller_character_2 (Utilities|Casting|CastToSideScrollerCharacter_2 OtherActor))
      (Variables|/Game/SideScrollerCPP/Blueprints/SideScrollerCharacter_2.SideScrollerCharacter_2_C|SetHealth _asside_scroller_character_2 (- (Variables|/Game/SideScrollerCPP/Blueprints/SideScrollerCharacter_2.SideScrollerCharacter_2_C|GetHealth _asside_scroller_character_2) 1e+01))
      (Development|PrintString "Hello")
      (Utilities|IsValid _s_ound_2
        (:Is%20Valid
          (Audio|Components|Audio|Play _s_ound_2 0.0))))))

(event OnComponentHit(Capsule)
  (params (HitComponent :type Primitive%20Component%20Object%20Reference) (OtherActor :type Actor%20Object%20Reference) (OtherComp :type Primitive%20Component%20Object%20Reference) (NormalImpulse :type Vector :default "0, 0, 0") (Hit :type Hit%20Result%20Structure%20%28by%20ref%29))
  (Utilities|Casting|CastToSideScrollerCharacter OtherActor)
  (if (not (Variables|Default|GetHasHit))
    (Variables|Default|SetHasHit true)
    (Class|AchievementSubSystem|AddAchievementProgress (Subsystems|GetAchievementSubSystem) "Barrel" 1.0)))

(event EventBeginPlay
  (bind _returnvalue (Audio|CreateSound2D "/Game/Sound/damaged1.damaged1" 1.0 1.0 0.0 0))
  (Variables|Default|SetS%20OUND _returnvalue))

(event Collision|EventActorBeginOverlap
  (params (OtherActor :type Actor%20Object%20Reference)))

(event EventTick
  (params (DeltaSeconds :type Float%20%28single-precision%29))
  (if (Variables|Default|GetCanRotate)
    (Transformation|AddActorLocalRotation "1.000000,0.000000, 0" false false)))

(fn ConstructionScript
  (Rendering|SetVisibility (Variables|Default|GetSpike) (Variables|Default|GetIsSpikesVisisble) false))