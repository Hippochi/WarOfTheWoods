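; Potion pickup for the side-scroller that is collected when either of the two player character classes overlaps its capsule.
; Each overlap advances the "Shield" achievement, plays a heal sound and increments the character's pickup count.
; Duplicated per-class branches then use a DoOnce to flag the character, update GameInstance and player stats, destroy the actor and play a 2D sound created at BeginPlay.
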(event OnComponentBeginOverlap(Capsule)
  (params (OverlappedComponent :type Primitive%20Component%20Object%20Reference) (OtherActor :type Actor%20Object%20Reference) (OtherComp :type Primitive%20Component%20Object%20Reference) (OtherBodyIndex :type Integer) (bFromSweep :type Boolean) (SweepResult :type Hit%20Result%20Structure%20%28by%20ref%29))
  (bind _asside_scroller_character (Utilities|Casting|CastToSideScrollerCharacter OtherActor)
    (:then
      (Class|AchievementSubSystem|AddAchievementProgress (Subsystems|GetAchievementSubSystem) "Shield" 1.0)
      (Audio|PlaySoundatLocation "/Game/Sound/healed2.healed2" "0, 0, 0" "0, 0, 0" 1.0 1.0 0.0 0 0 0)
      (bind _result (Math|Integer|IncrementInt (Variables|/Game/SideScrollerCPP/Blueprints/SideScrollerCharacter.SideScrollerCharacter_C|GetPickups _asside_scroller_character))
        (:%20%20
          (Variables|/Game/SideScrollerCPP/Blueprints/SideScrollerCharacter.SideScrollerCharacter_C|SetPickups _asside_scroller_character _result)
          (Utilities|FlowControl|DoOnce false
            (:Completed
              (Variables|/Game/SideScrollerCPP/Blueprints/SideScrollerCharacter.SideScrollerCharacter_C|SethasPickUp _asside_scroller_character true)
              (bind _asgame_instance_bp (Utilities|Casting|CastToGameInstanceBP (Game|GetGameInstance)))
              (Variables|/Game/SideScrollerCPP/Blueprints/GameInstanceBP.GameInstanceBP_C|SetPickUps _asgame_instance_bp (+ (Variables|/Game/SideScrollerCPP/Blueprints/GameInstanceBP.GameInstanceBP_C|GetPickUps _asgame_instance_bp) 1))
              (CallFunction|AddActivePlayerStats 0.0 0 1)
              (Actor|DestroyActor)
              (Audio|Components|Audio|Play (Variables|Default|GetPickupSound) 0.0))))))
    (:CastFailed
      (bind _asside_scroller_character_2 (Utilities|Casting|CastToSideScrollerCharacter_2 OtherActor))
      (Class|AchievementSubSystem|AddAchievementProgress (Subsystems|GetAchievementSubSystem) "Shield" 1.0)
      (Audio|PlaySoundatLocation "/Game/Sound/healed2.healed2" "0, 0, 0" "0, 0, 0" 1.0 1.0 0.0 0 0 0)
      (bind _result_2 (Math|Integer|IncrementInt (Variables|/Game/SideScrollerCPP/Blueprints/SideScrollerCharacter_2.SideScrollerCharacter_2_C|GetPickups _asside_scroller_character_2))
        (:%20%20
          (Variables|/Game/SideScrollerCPP/Blueprints/SideScrollerCharacter_2.SideScrollerCharacter_2_C|SetPickups _asside_scroller_character_2 _result_2)
          (Utilities|FlowControl|DoOnce false
            (:Completed
              (Variables|/Game/SideScrollerCPP/Blueprints/SideScrollerCharacter_2.SideScrollerCharacter_2_C|SethasPickUp _asside_scroller_character_2 true)
              (bind _asgame_instance_bp_2 (Utilities|Casting|CastToGameInstanceBP (Game|GetGameInstance)))
              (Variables|/Game/SideScrollerCPP/Blueprints/GameInstanceBP.GameInstanceBP_C|SetPickUps _asgame_instance_bp_2 (+ (Variables|/Game/SideScrollerCPP/Blueprints/GameInstanceBP.GameInstanceBP_C|GetPickUps _asgame_instance_bp_2) 1))
              (CallFunction|AddActivePlayerStats 0.0 0 1)
              (Actor|DestroyActor)
              (Audio|Components|Audio|Play (Variables|Default|GetPickupSound) 0.0))))))))

(event EventBeginPlay
  (bind _returnvalue (Audio|CreateSound2D "/Game/Core/Asset/Sound/Pickup.Pickup" 1.0 1.0 0.0 0))
  (Variables|Default|SetPickupSound _returnvalue))

(fn ConstructionScript)