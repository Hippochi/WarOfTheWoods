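; Bear trap hazard that damages either side-scroller character on overlap, snaps it to the box center and disables its movement.
; Timelines close the two claws, one timeline per character class, with the Oldman flag recording the second class.
; Repeated gamepad top-button or E presses, reset after a short pause, reverse the claws and restore walking; E only runs the first character's release.
; The trigger box re-arms after a delay.
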(event OnComponentBeginOverlap(Box)
  (params (OverlappedComponent :type Primitive%20Component%20Object%20Reference) (OtherActor :type Actor%20Object%20Reference) (OtherComp :type Primitive%20Component%20Object%20Reference) (OtherBodyIndex :type Integer) (bFromSweep :type Boolean) (SweepResult :type Hit%20Result%20Structure%20%28by%20ref%29))
  (bind _asside_scroller_character (Utilities|Casting|CastToSideScrollerCharacter OtherActor)
    (:then
      (Variables|/Game/SideScrollerCPP/Blueprints/SideScrollerCharacter.SideScrollerCharacter_C|SetHealth _asside_scroller_character (- (Variables|/Game/SideScrollerCPP/Blueprints/SideScrollerCharacter.SideScrollerCharacter_C|GetHealth _asside_scroller_character) 1e+01))
      (Variables|Default|SetOldman false)
      (CallFunction|CatchPlayer _asside_scroller_character)
      (Input|EnableInput (Game|GetPlayerController 0))
      (Collision|SetCollisionEnabled (Variables|Default|GetBox) "NoCollision")
      (bind _track (Timeline|OpenClose Play)
        (:Update
          (Transformation|SetRelativeRotation (Variables|Default|GetRightClaw) (Math|Rotator|MakeRotator 0.0 (Math|Float|Lerp 0.0 6e+01 _track) 0.0) false false)
          (Transformation|SetRelativeRotation (Variables|Default|GetLeftClaw) (Math|Rotator|MakeRotator 0.0 (Math|Float|Lerp 0.0 -6e+01 _track) 0.0) false false))))
    (:CastFailed
      (bind _asside_scroller_character_2 (Utilities|Casting|CastToSideScrollerCharacter_2 OtherActor))
      (Variables|/Game/SideScrollerCPP/Blueprints/SideScrollerCharacter_2.SideScrollerCharacter_2_C|SetHealth _asside_scroller_character_2 (- (Variables|/Game/SideScrollerCPP/Blueprints/SideScrollerCharacter_2.SideScrollerCharacter_2_C|GetHealth _asside_scroller_character_2) 1e+01))
      (Variables|Default|SetOldman true)
      (CallFunction|CatchPlayer _asside_scroller_character_2)
      (Input|EnableInput (Game|GetPlayerController 0))
      (Collision|SetCollisionEnabled (Variables|Default|GetBox) "NoCollision")
      (bind _track_2 (Timeline|Timeline_0 Play)
        (:Update
          (Transformation|SetRelativeRotation (Variables|Default|GetRightClaw) (Math|Rotator|MakeRotator 0.0 (Math|Float|Lerp 0.0 6e+01 _track_2) 0.0) false false)
          (Transformation|SetRelativeRotation (Variables|Default|GetLeftClaw) (Math|Rotator|MakeRotator 0.0 (Math|Float|Lerp 0.0 -6e+01 _track_2) 0.0) false false))))))

(event Custom|CatchPlayer
  (params (Character :type Character%20Object%20Reference))
  (bind _box (Variables|Default|GetBox))
  (bind _returnvalue (Transformation|GetWorldLocation _box))
  (Pawn|Components|CharacterMovement|DisableMovement (Variables|/Script/Engine.Character|GetCharacterMovement Character))
  (Transformation|SetActorLocation Character (Math|Vector|MakeVector (.x _returnvalue) (.y _returnvalue) (.z (Transformation|GetActorLocation Character))) false false))

(event Custom|OpenTrap
  (Pawn|Components|CharacterMovement|SetMovementMode (Variables|/Script/Engine.Character|GetCharacterMovement (stale OnComponentBeginOverlap(Box) _asside_scroller_character_2)) "MOVE_Walking" 0)
  (Utilities|FlowControl|Sequence
    (:then_0
      (bind _track (Timeline|Timeline_0 Reverse)
        (:Update
          (Transformation|SetRelativeRotation (Variables|Default|GetRightClaw) (Math|Rotator|MakeRotator 0.0 (Math|Float|Lerp 0.0 6e+01 _track) 0.0) false false)
          (Transformation|SetRelativeRotation (Variables|Default|GetLeftClaw) (Math|Rotator|MakeRotator 0.0 (Math|Float|Lerp 0.0 -6e+01 _track) 0.0) false false))))
    (:then_1
      (Utilities|FlowControl|Delay 2.0)
      (Collision|SetCollisionEnabled (Variables|Default|GetBox) "QueryAndPhysics"))))

(event Custom|Open
  (Pawn|Components|CharacterMovement|SetMovementMode (Variables|/Script/Engine.Character|GetCharacterMovement (stale OnComponentBeginOverlap(Box) _asside_scroller_character)) "MOVE_Walking" 0)
  (Utilities|FlowControl|Sequence
    (:then_0
      (bind _track (Timeline|OpenClose Reverse)
        (:Update
          (Transformation|SetRelativeRotation (Variables|Default|GetRightClaw) (Math|Rotator|MakeRotator 0.0 (Math|Float|Lerp 0.0 6e+01 _track) 0.0) false false)
          (Transformation|SetRelativeRotation (Variables|Default|GetLeftClaw) (Math|Rotator|MakeRotator 0.0 (Math|Float|Lerp 0.0 -6e+01 _track) 0.0) false false))))
    (:then_1
      (Utilities|FlowControl|Delay 2.0)
      (Collision|SetCollisionEnabled (Variables|Default|GetBox) "QueryAndPhysics"))))

(event Input|KeyboardEvents|E
  (params (Key :type Key%20Structure :default "None"))
  (:Pressed
    (bind _result (Math|Integer|IncrementInt (Variables|Default|GetPresses))
      (:%20%20
        (if (== _result (Variables|Default|GetPressesNeeded))
          (CallFunction|Open)))))
  (:Released
    (Utilities|FlowControl|RetriggerableDelay 0.5)
    (Variables|Default|SetPresses 0)))

(event Input|GamepadEvents|GamepadFaceButtonTop
  (params (Key :type Key%20Structure :default "None"))
  (:Pressed
    (bind _result (Math|Integer|IncrementInt (Variables|Default|GetPresses))
      (:%20%20
        (if (== _result (Variables|Default|GetPressesNeeded))
          (if (Variables|Default|GetOldman)
            (CallFunction|OpenTrap)
            (else
              (CallFunction|Open)))))))
  (:Released
    (Utilities|FlowControl|RetriggerableDelay 0.5)
    (Variables|Default|SetPresses 0)))

(fn ConstructionScript)